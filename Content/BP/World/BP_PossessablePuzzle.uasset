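; Base possessable puzzle that the player interacts with to take control, exposing interactable and solved status.
; Interact blocks player movement, saves control rotation, smooth-possesses the puzzle facing its camera and pushes a CAW_Possessable widget.
; Move input resolves by dominant axis into empty Left, Right, Up and Down events, gated on CanInteract.
; Leave or the interact input removes the widget, smooth-possesses the player back and restores rotation and movement, guarded by a DoOnce.
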(event `self.ReceiveBeginPlay`
  (set `self.Activatable Widget Class` "/Game/UI/CAW_Possessable.CAW_Possessable_C"))

(event `/Game/BP/Interfaces/BPI_Interact.Interact`
  (params (Sender :type "Actor Object Reference"))
  (bind _returnvalue (`GameplayStatics.GetPlayerController` 0))
  (bind _asbp_player (cast `/Game/BP/Core/BP_Player` Sender))
  (bind _output_get (set `self.PlayerRef` _asbp_player))
  (`/Engine/EditorBlueprintResources/StandardMacros.IncrementInt` (`/Game/BP/Core/BP_Player.CanMove` _output_get)
    (:`  `
      (set `self.ControlRotation` (`self.GetControlRotation` (`self.PlayerRef`)))
      (`/Game/BP/Libraries/ML_Utils.SmoothPossess` (`GameplayStatics.GetPlayerController` 0) self)
      (`Controller.SetControlRotation` _returnvalue (`SceneComponent.K2_GetComponentRotation` (`self.Camera`)))
      (bind _returnvalue_2 (`CommonActivatableWidgetContainerBase.BP_AddWidget` (`/Game/BP/Libraries/ML_Utils.ReturnMainStack` _returnvalue) (`self.Activatable Widget Class`)))
      (set `self.ActiveWidget` _returnvalue_2))))

(event `Leave`
  (`/Engine/EditorBlueprintResources/StandardMacros.DoOnce` false :!label _label
    (:`Completed`
      (`CommonActivatableWidgetContainerBase.RemoveWidget` (`/Game/BP/Libraries/ML_Utils.ReturnMainStack` (`GameplayStatics.GetPlayerController` 0)) (`self.ActiveWidget`))
      (`/Game/BP/Libraries/ML_Utils.SmoothPossess` (`GameplayStatics.GetPlayerController` 0) (`self.PlayerRef`))
      (`Controller.SetControlRotation` (`GameplayStatics.GetPlayerController` 0) (`self.ControlRotation`))
      (`/Engine/EditorBlueprintResources/StandardMacros.DecrementInt` (`/Game/BP/Core/BP_Player.CanMove` (`self.PlayerRef`))
        (:`  `
          (goto _label :!via `Reset`))))))

(event `EnhancedInput|/Game/Input/IA_Interact`
  (params (ActionValue :type Boolean) (ElapsedSeconds :type "Float (double-precision)") (TriggeredSeconds :type "Float (double-precision)") (InputAction :type "InputAction Object Reference" :default "/Game/Input/IA_Interact.IA_Interact"))
  (:`Started`
    (goto _label)))

(event `EnhancedInput|/Game/Input/IA_Jump`
  (params (ActionValue :type Boolean) (ElapsedSeconds :type "Float (double-precision)") (TriggeredSeconds :type "Float (double-precision)") (InputAction :type "InputAction Object Reference" :default "/Game/Input/IA_Jump.IA_Jump")))

(event `EnhancedInput|/Game/Input/IA_Move`
  (params (ActionValue :type "Vector2D Structure") (ElapsedSeconds :type "Float (double-precision)") (TriggeredSeconds :type "Float (double-precision)") (InputAction :type "InputAction Object Reference" :default "/Game/Input/IA_Move.IA_Move"))
  (bind (_x _y) (`KismetMathLibrary.BreakVector2D` ActionValue))
  (:`Started`
    (`self.bCanInteract`
      (:`then`
        (if (> (`KismetMathLibrary.Abs` _x) (`KismetMathLibrary.Abs` _y))
          (`/Engine/EditorBlueprintResources/StandardMacros.CompareFloat` _x
            (:`>`
              (`self.Right`))
            (:`<`
              (`self.Left`)))
          (else
            (`/Engine/EditorBlueprintResources/StandardMacros.CompareFloat` _y
              (:`>`
                (`self.Up`))
              (:`<`
                (`self.Down`))))))
      (:`else`))))

(event `Left`)

(event `Right`)

(event `Up`)

(event `Down`)

(fn `ReturnInteractStatus`
  (returns (Interactable :type Boolean))
  (return (`self.Interactable`)))

(fn `ReturnSolvedStatus`
  (returns (Solved :type Boolean))
  (return (`self.Solved`)))

(fn `UserConstructionScript`)