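; BP_Telefon is an interactable telephone that rings and plays dialogue when answered.
; Interact stops the ring, pushes a dialogue widget onto the main UI stack with UI-only input, and shows lines from DT_DialogueOptions keyed by the manager's current dialogue key.
; NextLine steps through the lines and closes after the last, restoring game input.
; Closing the "Intro" dialogue advances the manager's key to "Room1".
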(event `self.ReceiveBeginPlay`)

(event `Ring`
  (`AudioComponent.Play` (`self.Audio`) 0.0))

(event `/Game/BP/Interfaces/BPI_Interact.Interact`
  (params (Sender :type "Actor Object Reference"))
  (bind _returnvalue (`GameplayStatics.GetPlayerController` 0))
  ;[0.15 0.008491 0 0.5] Interact
  (`AudioComponent.Stop` (`self.Audio`))
  (set `self.IsDialogueActive` true)
  (bind _output_get (set `self.CurrentDialogueKey` (`/Game/BP/World/BP_DialogueManager.CurrentDialogueKey` (`self.Managerref`))))
  (set `self.CurrentLineIndex` 0)
  (`KismetSystemLibrary.PrintString` (`KismetStringLibrary.Conv_NameToString` _output_get))
  (bind _returnvalue_2 (`CommonActivatableWidgetContainerBase.BP_AddWidget` (`/Game/BP/Libraries/ML_Utils.ReturnMainStack` _returnvalue) "/Game/UI/CAW_Dialogue.CAW_Dialogue_C"))
  (bind _output_get_2 (set `self.UI_Ref` _returnvalue_2))
  (`WidgetBlueprintLibrary.SetInputMode_UIOnlyEx` _returnvalue _output_get_2)
  (set `/Game/UI/CAW_Dialogue.Telefon` self _output_get_2)
  (set `PlayerController.bShowMouseCursor` true _returnvalue)
  (bind _returnvalue_3 (`|GetDataTableRow` "/Game/BP/World/DT_DialogueOptions.DT_DialogueOptions" (`self.CurrentDialogueKey`))
    (:`then`
      (`/Game/UI/CAW_Dialogue.SetDialogueText` (`self.UI_Ref`) (`|GetArrayItem` (`.Lines_3_962AF81442545CAB6049D8B145D5D503` (break `/Game/BP/World/S_DialogueLines` _returnvalue_3)) (`self.CurrentLineIndex`))))))

(event `CloseDialogue`
  (bind _returnvalue (`GameplayStatics.GetPlayerController` 0))
  ;[0.15 0.03031 0 0.5] Close Dialogue
  (`CommonActivatableWidgetContainerBase.RemoveWidget` (`/Game/BP/Libraries/ML_Utils.ReturnMainStack` _returnvalue) (`self.UI_Ref`) :!label _label)
  (`WidgetBlueprintLibrary.SetInputMode_GameOnly` _returnvalue true)
  (set `PlayerController.bShowMouseCursor` false _returnvalue)
  (if (== (`self.CurrentDialogueKey`) "Intro")
    (set `/Game/BP/World/BP_DialogueManager.CurrentDialogueKey` "Room1" (`self.Managerref`))
    (set `self.DialogueEnded` true)
    (set `self.IsDialogueActive` false)))

(event `NextLine`
  (`KismetSystemLibrary.PrintString` "next line")
  (bind _returnvalue (`|GetDataTableRow` "/Game/BP/World/DT_DialogueOptions.DT_DialogueOptions" (`self.CurrentDialogueKey`))
    (:`then`
      (bind _result (`/Engine/EditorBlueprintResources/StandardMacros.IncrementInt` (`self.CurrentLineIndex`))
        (:`  `
          (if (>= _result (`KismetArrayLibrary.Array_Length` (`.Lines_3_962AF81442545CAB6049D8B145D5D503` (break `/Game/BP/World/S_DialogueLines` _returnvalue))))
            (goto _label)
            (else
              ;[0.15 0.05243 0.000305 0.5] Update Line
              (bind _returnvalue_2 (`|GetDataTableRow` "/Game/BP/World/DT_DialogueOptions.DT_DialogueOptions" (`self.CurrentDialogueKey`))
                (:`then`
                  (`/Game/UI/CAW_Dialogue.SetDialogueText` (`self.UI_Ref`) (`|GetArrayItem` (`.Lines_3_962AF81442545CAB6049D8B145D5D503` (break `/Game/BP/World/S_DialogueLines` _returnvalue_2)) (`self.CurrentLineIndex`))))))))))))

(fn `ReturnInteractStatus`
  (returns (Interactable :type Boolean))
  (locals (NewLocalVar :type Boolean :default true))
  (return (`self.Interactable`)))

(fn `UserConstructionScript`)