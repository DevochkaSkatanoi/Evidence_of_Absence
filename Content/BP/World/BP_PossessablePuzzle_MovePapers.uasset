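; Possessable puzzle in which directional events slide the SideB component, by its name one of a set of papers, into a solved position.
; Up, Down, Left and Right nudge it along Z and Y within bounds the construction script centers on its start.
; Each move runs a tolerance check, delayed for horizontal moves; a match sets the solved flag, notifies ActorToReact and calls Leave.
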(event `self.Up`
  (if (< (.z (`SceneComponent.RelativeLocation` (`self.SideB`))) (.z (`self.PositiveBoundaries`)))
    (`SceneComponent.K2_AddRelativeLocation` (`self.SideB`) (0.0 0.0 1.0) false false)
    (`self.SolvedCheck`)))

(event `self.Down`
  (if (> (.z (`SceneComponent.RelativeLocation` (`self.SideB`))) (.z (`self.NegativeBoundaries`)))
    (`SceneComponent.K2_AddRelativeLocation` (`self.SideB`) (0.0 0.0 -1.0) false false)
    (`self.SolvedCheck`)))

(event `self.Right`
  (if (< (.y (`SceneComponent.RelativeLocation` (`self.SideB`))) (.y (`self.PositiveBoundaries`)))
    (`SceneComponent.K2_AddRelativeLocation` (`self.SideB`) (0.0 1.0 0.0) false false)
    (`KismetSystemLibrary.Delay` 0.2)
    (`self.SolvedCheck`)))

(event `self.Left`
  (if (> (.y (`SceneComponent.RelativeLocation` (`self.SideB`))) (.y (`self.NegativeBoundaries`)))
    (`SceneComponent.K2_AddRelativeLocation` (`self.SideB`) (0.0 -1.0 0.0) false false)
    (`KismetSystemLibrary.Delay` 0.2)
    (`self.SolvedCheck`)))

(event `SolvedCheck`
  (if (and (`KismetMathLibrary.NearlyEqual_FloatFloat` (.y (`SceneComponent.RelativeLocation` (`self.SideB`))) (.y (`self.SilvedPosition`)) 0.1) (`KismetMathLibrary.NearlyEqual_FloatFloat` (.z (`SceneComponent.RelativeLocation` (`self.SideB`))) (.z (`self.SilvedPosition`)) 0.1))
    (`KismetSystemLibrary.PrintString` "Solved")
    (set `self.Solved_0` true)
    (message `/Game/BP/Interfaces/BPI_React.React` (`self.ActorToReact`) true "None")
    (`self.Leave`)))

(fn `ReturnSolvedStatus`
  (returns (Solved :type Boolean))
  (return (`self.Solved_0`)))

(fn `UserConstructionScript`
  (`parent.UserConstructionScript`)
  (bind _output_get (set `self.OffsetPosition` (`SceneComponent.RelativeLocation` (`self.SideB`))))
  (set `self.PositiveBoundaries` (+ _output_get (20.0 20.0 20.0)))
  (set `self.NegativeBoundaries` (- _output_get (20.0 20.0 20.0))))