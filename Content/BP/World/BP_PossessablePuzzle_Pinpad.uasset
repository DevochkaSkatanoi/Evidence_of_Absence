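; Possessable pinpad puzzle where the player enters a button sequence on a grid of four rows and three columns.
; Directional events move a wrapping cursor shown by an outline overlay material, and IA_Jump selects each button once, swapping its material.
; At full length the entry is compared in order with CorrectSequence.
; A match notifies ActorToReact and calls Leave, while a mismatch resets selections and cursor.
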(event `self.Down`
  (bind _returnvalue (+ (`self.CurrentRow`) 1))
  (set `self.CurrentRow` (`KismetMathLibrary.SelectInt` 0 _returnvalue (> _returnvalue (`KismetArrayLibrary.Array_LastIndex` (`self.Buttons`)))))
  (`self.HighlightButton` true))

(event `self.Up`
  (bind _returnvalue (- (`self.CurrentRow`) 1))
  (set `self.CurrentRow` (`KismetMathLibrary.SelectInt` (`KismetArrayLibrary.Array_LastIndex` (`self.Buttons`)) _returnvalue (< _returnvalue 0)))
  (`self.HighlightButton` true))

(event `self.Right`
  (bind _returnvalue (+ (`self.CurrentColumn`) 1))
  (set `self.CurrentColumn` (`KismetMathLibrary.SelectInt` 0 _returnvalue (> _returnvalue (`KismetArrayLibrary.Array_LastIndex` (`.Meshes_4_DB1D248F4FEF5B890D6485A11AF039DE` (break `/Game/BP/World/S_Symbols` (`|GetArrayItem` (`self.Buttons`) (`self.CurrentRow`))))))))
  (`self.HighlightButton` true))

(event `self.Left`
  (bind _returnvalue (- (`self.CurrentColumn`) 1))
  (set `self.CurrentColumn` (`KismetMathLibrary.SelectInt` (`KismetArrayLibrary.Array_LastIndex` (`.Meshes_4_DB1D248F4FEF5B890D6485A11AF039DE` (break `/Game/BP/World/S_Symbols` (`|GetArrayItem` (`self.Buttons`) (`self.CurrentRow`))))) _returnvalue (< _returnvalue 0)))
  (`self.HighlightButton` true))

(event `EnhancedInput|/Game/Input/IA_Jump`
  (params (ActionValue :type Boolean) (ElapsedSeconds :type "Float (double-precision)") (TriggeredSeconds :type "Float (double-precision)") (InputAction :type "InputAction Object Reference" :default "/Game/Input/IA_Jump.IA_Jump"))
  (bind _s_buttonindex (make `/Game/BP/World/S_ButtonIndex` (`self.CurrentRow`) (`self.CurrentColumn`)))
  (:`Started`
    (if (not (`self.Solved`))
      (if (not (`KismetArrayLibrary.Array_Contains` (`self.SelectedButtons`) (make `/Game/BP/World/S_ButtonIndex` (`self.CurrentRow`) (`self.CurrentColumn`))))
        (`KismetArrayLibrary.Array_Add` (`self.PlayerSequence`) _s_buttonindex)
        (`KismetArrayLibrary.Array_Add` (`self.SelectedButtons`) _s_buttonindex)
        (`PrimitiveComponent.SetMaterial` (`|GetArrayItem` (`.Meshes_4_DB1D248F4FEF5B890D6485A11AF039DE` (break `/Game/BP/World/S_Symbols` (`|GetArrayItem` (`self.Buttons`) (`self.CurrentRow`)))) (`self.CurrentColumn`)) 0 "/Game/Materials/Material_Textures/MI_SafeNumbers_Highlight.MI_SafeNumbers_Highlight")
        (if (== (`KismetArrayLibrary.Array_Length` (`self.CorrectSequence`)) (`KismetArrayLibrary.Array_Length` (`self.PlayerSequence`)))
          (if (`KismetArrayLibrary.Array_Identical` (`self.CorrectSequence`) (`self.PlayerSequence`))
            (set `self.Solved_0` true)
            (`KismetSystemLibrary.PrintString` "SOLVED" true true (struct :`R` 1.0 :`B` 0.694978 :`A` 1.0) 5.0)
            (message `/Game/BP/Interfaces/BPI_React.React` (`self.ActorToReact`) true "None")
            (`self.Leave`)
            (else
              (`self.ResetPuzzle`))))))))

(event `ResetPuzzle`
  (`KismetArrayLibrary.Array_Clear` (`self.PlayerSequence`))
  (`KismetArrayLibrary.Array_Clear` (`self.SelectedButtons`))
  (for _array_element (`self.Buttons`)
    (for _array_element_2 (`.Meshes_4_DB1D248F4FEF5B890D6485A11AF039DE` (break `/Game/BP/World/S_Symbols` _array_element))
      (`PrimitiveComponent.SetMaterial` _array_element_2 0 "/Game/Materials/Material_Textures/MI_SafeNumbers.MI_SafeNumbers")
      (set `self.CurrentRow` 0)
      (set `self.CurrentColumn` 0)
      (`self.HighlightButton` true))))

(fn `HighlightButton`
  (params (EnableHighlight :type Boolean))
  (for _array_element (`self.Buttons`)
    (for _array_element_2 (`.Meshes_4_DB1D248F4FEF5B890D6485A11AF039DE` (break `/Game/BP/World/S_Symbols` _array_element))
      (`MeshComponent.SetOverlayMaterial` _array_element_2 null)))
  (if EnableHighlight
    (`MeshComponent.SetOverlayMaterial` (`|GetArrayItem` (`.Meshes_4_DB1D248F4FEF5B890D6485A11AF039DE` (break `/Game/BP/World/S_Symbols` (`|GetArrayItem` (`self.Buttons`) (`self.CurrentRow`)))) (`self.CurrentColumn`)) "/Game/Materials/M_Outline_3.M_Outline_3")))

(fn `IsButtonSelected`
  (params (Row :type Integer) (Column :type Integer))
  (returns (REturnValue :type Boolean))
  (return (`KismetArrayLibrary.Array_Contains` (`self.SelectedButtons`) (make `/Game/BP/World/S_ButtonIndex` Row Column))))

(fn `ReturnSolvedStatus`
  (returns (Solved :type Boolean))
  (return (`self.Solved_0`)))

(fn `SetButtonSelected`
  (params (TargetMesh :type "StaticMeshComponent Object Reference"))
  (`PrimitiveComponent.SetMaterial` TargetMesh 0 "/Game/Materials/MI_Grid_Green.MI_Grid_Green"))

(fn `UserConstructionScript`
  (`parent.UserConstructionScript`)
  (bind _output_get (set `self.Buttons` (`|MakeArray` (make `/Game/BP/World/S_Symbols` (`|MakeArray` (`self.R0C0`) (`self.R0C1`) (`self.R0C2`))) (make `/Game/BP/World/S_Symbols` (`|MakeArray` (`self.R1C0`) (`self.R1C1`) (`self.R1C2`))) (make `/Game/BP/World/S_Symbols` (`|MakeArray` (`self.R2C0`) (`self.R2C1`) (`self.R2C2`))) (make `/Game/BP/World/S_Symbols` (`|MakeArray` (`self.R3C0`) (`self.R3C1`) (`self.R3C2`))))))
  (for _array_element _output_get
    (for _ (`.Meshes_4_DB1D248F4FEF5B890D6485A11AF039DE` (break `/Game/BP/World/S_Symbols` _array_element))
      (set `self.CurrentRow` 0)
      (set `self.CurrentColumn` 0)
      (`self.HighlightButton` true))))