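; Interactable hinged door that swings open and closed, optionally locked behind a held collectable with a matching ID.
; Player interaction checks Interactable and NeededID, optionally consumes the item, or shows HUD text on refusal; other senders and React skip these checks.
; A FlipFlop plays or reverses a timeline rotating MoveScene, with handle motion only while opening.
; Referenced objects attach to MoveScene at BeginPlay; an unused MoveComponentTo branch remains.
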(event `self.ReceiveBeginPlay`
  (set `self.StartTransform` (`SceneComponent.GetRelativeTransform` (`self.MoveScene`)))
  (for _array_element (`self.Object Refs`)
    (`self.K2_AttachToComponent` _array_element (`self.MoveScene`) "None" "KeepWorld" "KeepWorld" "KeepWorld" true)))

(event `/Game/BP/Interfaces/BPI_Interact.Interact`
  (params (Sender :type "Actor Object Reference"))
  (`KismetSystemLibrary.IsObjectOfSoftClass` Sender "/Game/BP/Core/BP_Player.BP_Player_C"
    (:`True`
      (bind _asbp_player (cast `/Game/BP/Core/BP_Player` Sender))
      ;[0.15 0.02244 8.3e-05 0.5] Check for ID
      (if (`self.Interactable`)
        (if (`KismetStringLibrary.IsEmpty` (`self.NeededID`))
          (set `self.Interactable` false :!label _label)
          (set `self.IsMoving` true)
          (`/Engine/EditorBlueprintResources/StandardMacros.FlipFlop` :!label _label_2
            (:`A`
              (bind (_direction _rotation _doormove) (`Timeline|HandleTimeline` :!label _label_3)
                (:`Update`
                  (`SceneComponent.K2_SetRelativeRotation` (`self.MoveScene`) (`KismetMathLibrary.MakeRotator` 0.0 0.0 (`KismetMathLibrary.Lerp` 0.0 (`self.DoorRotation`) _doormove)) false false)
                  (if (not (`TimelineComponent.IsReversing` (`self.HandleTimeline`)))
                    (`SceneComponent.K2_SetRelativeRotation` (`self.HandleMove`) (`KismetMathLibrary.MakeRotator` 0.0 (`KismetMathLibrary.Lerp` 0.0 20.0 _rotation)) false false)))
                (:`Finished`
                  (`self.MoveOnce`
                    (:`then`)
                    (:`else`
                      (set `self.Interactable` true)
                      (set `self.IsMoving` false))))))
            (:`B`
              (goto _label_3 :!via `Reverse`)))
          (else
            (bind _heldcollectable (`/Game/BP/Core/BP_Player.HeldCollectable` _asbp_player))
            (`/Engine/EditorBlueprintResources/StandardMacros.IsValid` _heldcollectable
              (:`Is Valid`
                (if (`KismetStringLibrary.EqualEqual_StrStr` (`/Game/BP/World/BP_Collectable.ID` _heldcollectable) (`self.NeededID`))
                  (`self.DestroyItem`
                    (:`then`
                      (set `self.NeededID` "")
                      (`self.K2_DestroyActor` (`/Game/BP/Core/BP_Player.HeldCollectable` _asbp_player))
                      (set `/Game/BP/Core/BP_Player.HeldCollectable` null _asbp_player)
                      (goto _label))
                    (:`else`
                      (goto _label)))
                  (else
                    _)))
              (:`Is Not Valid`
                _))
            ;[0.15 0.1452 0.009007 0.5] ToDo: text variations
            (bind _asbp_hud (cast `/Game/UI/BP_HUD` (`PlayerController.GetHUD` (`GameplayStatics.GetPlayerController` 0))))
            (`/Game/UI/BP_HUD.IngameText` _asbp_hud (`self.WrongItem`))))
        (elif (not (`self.IsMoving`))
          (bind _asbp_hud_2 (cast `/Game/UI/BP_HUD` (`PlayerController.GetHUD` (`GameplayStatics.GetPlayerController` 0))))
          (`/Game/UI/BP_HUD.IngameText` _asbp_hud_2 (`self.Locked`)))))
    (:`False`
      (goto _label))))

(event `/Game/BP/Interfaces/BPI_React.React`
  (params (Solved :type Boolean) (DialogueKey :type Name))
  (goto _label_2))

(fn `ReturnInteractStatus`
  (returns (Interactable :type Boolean))
  (return true))

(fn `UserConstructionScript`)