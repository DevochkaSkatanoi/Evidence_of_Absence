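; BP_InteractableEvidence is a world pickup that unlocks a piece of evidence when the player interacts with it.
; Interact records its EvidenceID in the player controller's UnlockedEvidences map and fires the evidence-unlocked notification.
; It then hides the mesh, disables its collision, deactivates the Niagara effect and shows its text through BP_HUD's IngameText.
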(event `/Game/BP/Interfaces/BPI_Interact.Interact`
  (params (Sender :type "Actor Object Reference"))
  (bind _evidenceid (`self.EvidenceID`))
  (bind _asbp_player_controller (cast `/Game/BP/Core/BP_PlayerController` (`GameplayStatics.GetPlayerController` 0)))
  (`BlueprintMapLibrary.Map_Add` (`/Game/BP/Core/BP_PlayerController.UnlockedEvidences` _asbp_player_controller) _evidenceid true)
  (`/Game/BP/Core/BP_PlayerController.OnEvidenceUnlocked` _asbp_player_controller _evidenceid)
  (`SceneComponent.SetVisibility` (`self.Mesh`) false false)
  (`PrimitiveComponent.SetCollisionEnabled` (`self.Mesh`) "NoCollision")
  (`ActorComponent.SetActive` (`self.Niagara`) false false)
  (bind _asbp_hud (cast `/Game/UI/BP_HUD` (`PlayerController.GetHUD` (`GameplayStatics.GetPlayerController` 0))))
  (`/Game/UI/BP_HUD.IngameText` _asbp_hud (`self.Text to Display`)))

(fn `UserConstructionScript`
  (`parent.UserConstructionScript`))