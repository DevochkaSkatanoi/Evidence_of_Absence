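; BP_Collectable is an interactable world item that the player can pick up and carry one at a time.
; Interact registers it as the player's HeldCollectable, disables collision and, after a short delay, snaps it to CollectablePivot.
; Pickup also turns off shadows and Niagara effects, fires the collected dispatcher and shows its text on the HUD.
; PlaceInSocket restores collision and shadows, while a setter and getter expose the interactable flag.
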(event `/Game/BP/Interfaces/BPI_Interact.Interact`
  (params (Sender :type "Actor Object Reference"))
  (bind _asbp_player (cast `/Game/BP/Core/BP_Player` Sender)) ; Если объект и так всегда будет загружен в сцене (игрок, HUD, Gamemode), \nто каст можно использовать. Если объект не загружен в сцене, то каст будет его \nпостоянно грузить и жрать оперативку
  (`/Game/BP/Core/BP_Player.HeldCollectable` _asbp_player
    (:`then`)
    (:`else`
      (set `/Game/BP/Core/BP_Player.HeldCollectable` self _asbp_player)
      (`PrimitiveComponent.SetCollisionEnabled` (`self.Mesh`) "NoCollision")
      (`KismetSystemLibrary.Delay` 0.2)
      (`self.K2_AttachToComponent` (`/Game/BP/Core/BP_Player.CollectablePivot` _asbp_player) "None" "SnapToTarget" "SnapToTarget" "SnapToTarget")
      (`PrimitiveComponent.SetCastShadow` (`self.Mesh`) false)
      (`self.OnCollectedDispatcher`)
      (bind _asbp_hud (cast `/Game/UI/BP_HUD` (`PlayerController.GetHUD` (`GameplayStatics.GetPlayerController` 0))))
      (`/Game/UI/BP_HUD.IngameText` _asbp_hud (`self.Full Text`))
      (`ActorComponent.SetActive` (`self.Niagara`) false false))))

(event `PlaceInSocket`
  (`PrimitiveComponent.SetCollisionEnabled` (`self.Mesh`) "QueryAndPhysics")
  (`PrimitiveComponent.SetCastShadow` (`self.Mesh`) true))

(event `/Game/BP/Interfaces/BPI_Interact.SetInteractStatus`
  (params (IsInteractable :type Boolean))
  (set `self.IsInteractable` IsInteractable))

(fn `ReturnInteractStatus`
  (returns (Interactable :type Boolean))
  (return (`self.IsInteractable`)))

(fn `UserConstructionScript`)