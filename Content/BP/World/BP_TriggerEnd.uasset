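; BP_TriggerEnd is a box trigger that plays the game's ending sequence when BP_Player overlaps it.
; It increments the player's CanMove counter, sends a solved ReactMessage to ActorToReact and plays footsteps and breathing.
; A chain of delays then times two ritual-reveal lines on BP_HUD, with a female whisper under the first.
; A final solved ReactMessage to the End reference closes the sequence.
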(event `self.Box.OnComponentBeginOverlap`
  (params (OverlappedComponent :type "PrimitiveComponent Object Reference") (OtherActor :type "Actor Object Reference") (OtherComp :type "PrimitiveComponent Object Reference") (OtherBodyIndex :type Integer) (bFromSweep :type Boolean) (SweepResult :type "HitResult Structure (by ref)"))
  (bind _asbp_player (cast `/Game/BP/Core/BP_Player` OtherActor))
  (`KismetSystemLibrary.Delay` 0.5)
  (`/Engine/EditorBlueprintResources/StandardMacros.IncrementInt` (`/Game/BP/Core/BP_Player.CanMove` _asbp_player)
    (:`  `
      (message `/Game/BP/Interfaces/BPI_React.React` (`self.ActorToReact`) true "None")
      (`GameplayStatics.PlaySound2D` "/Game/Audio/SFX/Footsteps_Wood/Footsteps_Wood_001.Footsteps_Wood_001" 1.0 1.0 0.0 null null)
      (`GameplayStatics.PlaySound2D` "/Game/Audio/SFX/Breathing.Breathing" 1.0 1.0 0.0 null null)
      (`KismetSystemLibrary.Delay` 7.0)
      (bind _asbp_hud (cast `/Game/UI/BP_HUD` (`PlayerController.GetHUD` (`GameplayStatics.GetPlayerController` 0))))
      (`/Game/UI/BP_HUD.IngameText` _asbp_hud "Thank you, Detective. You spent all this time searching for the truth... and in the end, you gave me exactly what I needed.")
      (`GameplayStatics.PlaySound2D` "/Game/Audio/SFX/female_whisper.female_whisper" 1.0 1.0 0.0 null null)
      (`KismetSystemLibrary.Delay` 5.0)
      (`/Game/UI/BP_HUD.IngameText` _asbp_hud "The ritual is complete now. He's waiting for me.")
      (`KismetSystemLibrary.Delay` 5.5)
      (message `/Game/BP/Interfaces/BPI_React.React` (`self.End`) true "None"))))

(fn `UserConstructionScript`)