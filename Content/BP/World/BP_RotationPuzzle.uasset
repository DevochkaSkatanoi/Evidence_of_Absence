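; Interactable rotation puzzle piece that steps through preset orientations and tells a linked actor when it reaches or leaves the solved one.
; Each interaction advances a wrapping index into RotationPoints, and a timeline lerps RotationScene there along the shortest path.
; When the timeline finishes, it updates the Solved flag and sends ReactMessage to ActorToReact, with a dialogue key on success.
; The construction script applies the starting rotation; getters expose interactable and solved status.
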(event `/Game/BP/Interfaces/BPI_Interact.Interact`
  (params (Sender :type "Actor Object Reference"))
  (bind _returnvalue (+ (`self.CurrentPositionIndex`) 1))
  (set `self.CurrentPositionIndex` (`KismetMathLibrary.SelectInt` 0 _returnvalue (> _returnvalue (`KismetArrayLibrary.Array_LastIndex` (`self.RotationPoints`)))))
  (bind _output_get (set `self.StartRotation` (`SceneComponent.RelativeRotation` (`self.RotationScene`))))
  (bind _output_get_2 (set `self.TargetRotation` (`|GetArrayItem` (`self.RotationPoints`) (`self.CurrentPositionIndex`))))
  (bind (_direction _rotation) (`Timeline|Timeline` :!via `PlayFromStart`)
    (:`Update`
      (`SceneComponent.K2_SetRelativeRotation` (`self.RotationScene`) (`KismetMathLibrary.RLerp` _output_get _output_get_2 _rotation true) true false))
    (:`Finished`
      (if (== (`self.CurrentPositionIndex`) (`self.SolvedPosIndex`))
        (set `self.Solved` true)
        (message `/Game/BP/Interfaces/BPI_React.React` (`self.ActorToReact`) true (`self.DialogueKey`))
        (else
          (`self.Solved` ; bool - convert to branch
            (:`then`
              (set `self.Solved` false)
              (message `/Game/BP/Interfaces/BPI_React.React` (`self.ActorToReact`) false "None"))
            (:`else`)))))))

(event `/Game/BP/Interfaces/BPI_Interact.SetInteractStatus`
  (params (IsInteractable :type Boolean))
  (set `self.Interactable` IsInteractable))

(fn `ReturnInteractStatus`
  (returns (Interactable :type Boolean))
  (return (`self.Interactable`)))

(fn `ReturnSolvedStatus`
  (returns (Solved :type Boolean))
  (return (`self.Solved`)))

(fn `UserConstructionScript`
  (`SceneComponent.K2_SetRelativeRotation` (`self.RotationScene`) (`|GetArrayItem` (`self.RotationPoints`) (`self.CurrentPositionIndex`)) false false))