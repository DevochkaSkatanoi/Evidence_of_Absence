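; BP_InteractableHint is an inspectable world object that can grant the player evidence and a hint when interacted with.
; Interact pushes an inspect widget onto the main UI stack, feeds it InspectData, and switches to UI-only input with the cursor shown.
; If UnlockEvidence is set, a DoOnce records both unlocks on BP_PlayerController, fires their notifications and shows text through BP_HUD.
; The construction script hardcodes the object's ID after calling its parent.
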(event `/Game/BP/Interfaces/BPI_Interact.Interact`
  (params (Sender :type "Actor Object Reference"))
  (bind _returnvalue (`GameplayStatics.GetPlayerController` 0))
  (bind _hintid (`self.HintID`))
  (bind _evidence_id (`self.Evidence ID`))
  (`KismetSystemLibrary.PrintString` "IntHint")
  (bind _returnvalue_2 (`CommonActivatableWidgetContainerBase.BP_AddWidget` (`/Game/BP/Libraries/ML_Utils.ReturnMainStack` (`GameplayStatics.GetPlayerController` 0)) "/Game/UI/CAW_InspectInteractable.CAW_InspectInteractable_C"))
  (`/Game/UI/CAW_InspectInteractable.InitializeInspect` _returnvalue_2 (`self.InspectData`))
  (`WidgetBlueprintLibrary.SetInputMode_UIOnlyEx` _returnvalue null)
  (set `PlayerController.bShowMouseCursor` true _returnvalue)
  (if (`self.bUnlockEvidence`)
    (`/Engine/EditorBlueprintResources/StandardMacros.DoOnce` false
      (:`Completed`
        (bind _asbp_player_controller (cast `/Game/BP/Core/BP_PlayerController` (`GameplayStatics.GetPlayerController` 0)))
        (`BlueprintMapLibrary.Map_Add` (`/Game/BP/Core/BP_PlayerController.UnlockedEvidences` _asbp_player_controller) _evidence_id true)
        (`/Game/BP/Core/BP_PlayerController.OnEvidenceUnlocked` _asbp_player_controller _evidence_id)
        (bind _asbp_hud (cast `/Game/UI/BP_HUD` (`PlayerController.GetHUD` (`GameplayStatics.GetPlayerController` 0))))
        (`/Game/UI/BP_HUD.IngameText` _asbp_hud (`self.Full Text_0`))
        (`BlueprintMapLibrary.Map_Add` (`/Game/BP/Core/BP_PlayerController.UnlockedHints` _asbp_player_controller) _hintid true)
        (`/Game/BP/Core/BP_PlayerController.OnHintUnlocked` _asbp_player_controller _hintid)
        (`KismetSystemLibrary.PrintString` "FunktionCalled")))))

(fn `UserConstructionScript`
  (`parent.UserConstructionScript`)
  (set `self.ID` "RedBox"))