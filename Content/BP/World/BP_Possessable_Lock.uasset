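; Possessable combination-lock puzzle with three rings: Up and Down select the outlined ring, Left and Right turn it.
; Each turn steps the ring's wrapping position index, and a timeline lerps it to the matching preset rotation.
; Every timeline update compares the indices to the correct combination.
; A match notifies the linked actor, hides the lock, calls Leave, and optionally destroys it after a delay.
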(event `self.ReceiveBeginPlay`
  (`parent.ReceiveBeginPlay`)
  (`KismetArrayLibrary.Array_Resize` (`self.CurrentPositionIndex`) (`KismetArrayLibrary.Array_Length` (`self.Rings`))))

(event `self.Down`
  (bind _returnvalue (+ (`self.CurrentRing`) 1))
  (set `self.CurrentRing` (`KismetMathLibrary.SelectInt` 0 _returnvalue (> _returnvalue (`KismetArrayLibrary.Array_LastIndex` (`self.Rings`)))))
  (`self.HighlightRing` true)
  (`KismetSystemLibrary.PrintString` "Down"))

(event `self.Up`
  (bind _returnvalue (- (`self.CurrentRing`) 1))
  (set `self.CurrentRing` (`KismetMathLibrary.SelectInt` (`KismetArrayLibrary.Array_LastIndex` (`self.Rings`)) _returnvalue (< _returnvalue 0)))
  (`self.HighlightRing` true)
  (`KismetSystemLibrary.PrintString` "Up"))

(event `self.Left`
  (bind _returnvalue (+ (`|GetArrayItem` (`self.CurrentPositionIndex`) (`self.CurrentRing`)) 1))
  (`KismetArrayLibrary.Array_Set` (`self.CurrentPositionIndex`) (`self.CurrentRing`) (`KismetMathLibrary.SelectInt` 0 _returnvalue (> _returnvalue (`KismetArrayLibrary.Array_LastIndex` (`self.RotationPoints`)))) true)
  (bind _output_get (set `self.StartRotation` (`SceneComponent.RelativeRotation` (`|GetArrayItem` (`self.Rings`) (`self.CurrentRing`)))))
  (bind _output_get_2 (set `self.TargetRotation` (`|GetArrayItem` (`self.RotationPoints`) (`|GetArrayItem` (`self.CurrentPositionIndex`) (`self.CurrentRing`)))))
  (set `self.bCanInteract` false)
  (bind (_direction _rotation) (`Timeline|Timeline` :!via `PlayFromStart`)
    (:`Update`
      (`SceneComponent.K2_SetRelativeRotation` (`|GetArrayItem` (`self.Rings`) (`self.CurrentRing`)) (`KismetMathLibrary.RLerp` _output_get _output_get_2 _rotation true) true false)
      (`self.SolvedCheck`))
    (:`Finished`
      (set `self.bCanInteract` true))))

(event `self.Right`
  (bind _returnvalue (- (`|GetArrayItem` (`self.CurrentPositionIndex`) (`self.CurrentRing`)) 1))
  (`KismetArrayLibrary.Array_Set` (`self.CurrentPositionIndex`) (`self.CurrentRing`) (`KismetMathLibrary.SelectInt` (`KismetArrayLibrary.Array_LastIndex` (`self.RotationPoints`)) _returnvalue (< _returnvalue 0)) true)
  (bind _output_get (set `self.StartRotation` (`SceneComponent.RelativeRotation` (`|GetArrayItem` (`self.Rings`) (`self.CurrentRing`)))))
  (bind _output_get_2 (set `self.TargetRotation` (`|GetArrayItem` (`self.RotationPoints`) (`|GetArrayItem` (`self.CurrentPositionIndex`) (`self.CurrentRing`)))))
  (set `self.bCanInteract` false)
  (bind (_direction _rotation) (`Timeline|Timeline_0` :!via `PlayFromStart`)
    (:`Update`
      (`SceneComponent.K2_SetRelativeRotation` (`|GetArrayItem` (`self.Rings`) (`self.CurrentRing`)) (`KismetMathLibrary.RLerp` _output_get _output_get_2 _rotation true) true false)
      (`self.SolvedCheck`))
    (:`Finished`
      (set `self.bCanInteract` true))))

(event `SolvedCheck`
  (if (== (`KismetArrayLibrary.Array_Length` (`self.CurrentPositionIndex`)) (`KismetArrayLibrary.Array_Length` (`self.CorrectPositionIndex`)))
    (if (`KismetArrayLibrary.Array_Identical` (`self.CurrentPositionIndex`) (`self.CorrectPositionIndex`))
      (set `self.Solved_0` true)
      (message `/Game/BP/Interfaces/BPI_React.React` (`self.ActorToReact`) true "None")
      (`SceneComponent.SetVisibility` (`self.Mesh`) false false)
      (for _array_element (`self.Rings`)
        (`SceneComponent.SetVisibility` _array_element false false))
      (`self.Leave`)
      (`KismetSystemLibrary.Delay` 1.0)
      (if (`self.DestroyAfterSolved`)
        (`self.K2_DestroyActor`)))))

(fn `HighlightRing`
  (params (EnableHighlight :type Boolean))
  (for (_array_element _array_index) (`self.Rings`)
    (if (== _array_index (`self.CurrentRing`))
      (`MeshComponent.SetOverlayMaterial` (`|GetArrayItem` (`self.Rings`) (`self.CurrentRing`)) "/Game/Materials/M_Outline_3.M_Outline_3")
      (else
        (`MeshComponent.SetOverlayMaterial` _array_element null)))))

(fn `ReturnSolvedStatus`
  (returns (Solved :type Boolean))
  (return (`self.Solved_0`)))

(fn `UserConstructionScript`
  (`parent.UserConstructionScript`)
  (`KismetArrayLibrary.Array_Clear` (`self.Rings`))
  (`KismetArrayLibrary.Array_Add` (`self.Rings`) (`self.R0`))
  (`KismetArrayLibrary.Array_Add` (`self.Rings`) (`self.R1`))
  (`KismetArrayLibrary.Array_Add` (`self.Rings`) (`self.R2`))
  (set `self.CurrentRing` 0)
  (`self.HighlightRing` true))