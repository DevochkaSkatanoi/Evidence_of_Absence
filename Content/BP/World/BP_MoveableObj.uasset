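; Interactable world object that eases a scene component, carrying its referenced components, between its start and target transforms on alternate triggers.
; Player interaction can require a held collectable with a matching ID, optionally destroyed to clear the requirement, otherwise showing an in-game text line.
; Non-player senders skip the ID check, and React triggers the move directly.
; Interact disables interaction, restored after the move unless it is move-once.
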(event `self.ReceiveBeginPlay`
  (set `self.StartTransform` (`SceneComponent.GetRelativeTransform` (`self.MoveScene`)))
  (for _array_element (`self.ObjectRefs`)
    (`self.K2_AttachToComponent` _array_element (`self.MoveScene`) "None" "KeepWorld" "KeepWorld" "KeepWorld" true)))

(event `self.Interact`
  (params (Sender :type "Actor Object Reference"))
  (bind _returnvalue (`GameplayStatics.GetPlayerController` 0))
  (`KismetSystemLibrary.IsObjectOfSoftClass` Sender "/Game/BP/Core/BP_Player.BP_Player_C"
    (:`True`
      ;[0.15 0.02244 8.3e-05 0.5] Check for ID
      (bind _asbp_player (cast `/Game/BP/Core/BP_Player` Sender))
      (if (`KismetStringLibrary.IsEmpty` (`self.NeededID`))
        (set `self.Interactable` false :!label _label)
        (bind _isa (`/Engine/EditorBlueprintResources/StandardMacros.FlipFlop` :!label _label_2)
          (:`A`
            _)
          (:`B`
            _))
        (`KismetSystemLibrary.MoveComponentTo` (`self.MoveScene`) (.location (`KismetMathLibrary.SelectTransform` (`self.TargetTransform`) (`self.StartTransform`) _isa)) (.rotation (`KismetMathLibrary.SelectTransform` (`self.TargetTransform`) (`self.StartTransform`) _isa)) true true (`self.MoveDuration`) true)
        (`self.MoveOnce`
          (:`then`)
          (:`else`
            (set `self.Interactable` true)))
        (else
          (bind _heldcollectable (`/Game/BP/Core/BP_Player.HeldCollectable` _asbp_player))
          (`/Engine/EditorBlueprintResources/StandardMacros.IsValid` _heldcollectable
            (:`Is Valid`
              (if (`KismetStringLibrary.EqualEqual_StrStr` (`/Game/BP/World/BP_Collectable.ID` _heldcollectable) (`self.NeededID`))
                (`self.DestroyItem`
                  (:`then`
                    (set `self.NeededID` "")
                    (`self.K2_DestroyActor` (`/Game/BP/Core/BP_Player.HeldCollectable` _asbp_player))
                    (set `/Game/BP/Core/BP_Player.HeldCollectable` null _asbp_player)
                    (goto _label))
                  (:`else`
                    (goto _label)))
                (else
                  _)))
            (:`Is Not Valid`
              _))
          (bind _returnvalue_2 (`CommonActivatableWidgetContainerBase.BP_AddWidget` (`/Game/BP/Libraries/ML_Utils.ReturnMainStack` _returnvalue) "/Game/UI/CAW_IngameLines.CAW_IngameLines_C"))
          (`WidgetBlueprintLibrary.SetInputMode_GameOnly` _returnvalue true)
          (set `/Game/UI/CAW_IngameLines.FullText` (`self.Full Text`) _returnvalue_2))))
    (:`False`
      (goto _label))))

(event `self.React`
  (params (Solved :type Boolean) (DialogueKey :type Name))
  (goto _label_2))

(fn `ReturnInteractStatus`
  (returns (Interactable :type Boolean))
  (return (`self.Interactable`)))

(fn `UserConstructionScript`)