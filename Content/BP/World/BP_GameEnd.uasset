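; BP_GameEnd is a world Blueprint that ends the game when its React event receives a solved state.
; It sets ShowCredits on BP_GameInstance, then adds the menu and credits widgets to the player's main widget stack.
; Finally, it shows the mouse cursor and opens MainLevel, with the credits flag held on the game instance across the level load.
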(event `/Game/BP/Interfaces/BPI_React.React`
  (params (Solved :type Boolean) (DialogueKey :type Name))
  (bind _returnvalue (`GameplayStatics.GetPlayerController` 0))
  (if Solved
    (bind _asbp_game_instance (cast `/Game/BP/Core/BP_GameInstance` (`GameplayStatics.GetGameInstance`)))
    (set `/Game/BP/Core/BP_GameInstance.ShowCredits` true _asbp_game_instance)
    (`CommonActivatableWidgetContainerBase.BP_AddWidget` (`/Game/BP/Libraries/ML_Utils.ReturnMainStack` (`GameplayStatics.GetPlayerController` 0)) "/Game/UI/CAW_Menu.CAW_Menu_C")
    (`CommonActivatableWidgetContainerBase.BP_AddWidget` (`/Game/BP/Libraries/ML_Utils.ReturnMainStack` _returnvalue) "/Game/UI/CAW_Credits.CAW_Credits_C")
    (set `PlayerController.bShowMouseCursor` true _returnvalue)
    (`GameplayStatics.OpenLevelBySoftObjectPtr` "/Game/Maps/MainLevel.MainLevel")))

(fn `UserConstructionScript`)