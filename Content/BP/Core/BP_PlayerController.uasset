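; BP_PlayerController is the player controller that opens the pause menu and detective board from Enhanced Input actions.
; On BeginPlay it adds the default mapping context and caches a reference to the first BP_Telefon in the level.
; Both actions push widgets onto the main stack and switch to UI-only input with a visible cursor; pause also freezes the game and centers the mouse.
; Opening the board fires a notification call and shows a first-time tutorial once.
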(event `self.ReceiveBeginPlay`
  (`EnhancedInputSubsystemInterface.AddMappingContext` (subsystem `EnhancedInputLocalPlayerSubsystem`) "/Game/Input/IMC_Default.IMC_Default" 0 (struct))
  (bind _outactors (`GameplayStatics.GetAllActorsOfClass` "/Game/BP/World/BP_Telefon.BP_Telefon_C"))
  (set `self.TelefonRef` (`|GetArrayItem` _outactors)))

(event `EnhancedInput|/Game/Input/IA_Pause`
  (params (ActionValue :type Boolean) (ElapsedSeconds :type "Float (double-precision)") (TriggeredSeconds :type "Float (double-precision)") (InputAction :type "InputAction Object Reference" :default "/Game/Input/IA_Pause.IA_Pause"))
  (bind (_x _y) (`KismetMathLibrary.BreakVector2D` (`WidgetLayoutLibrary.GetViewportSize`)))
  (:`Started`
    (`GameplayStatics.SetGamePaused` true)
    (bind _returnvalue (`CommonActivatableWidgetContainerBase.BP_AddWidget` (`/Game/BP/Libraries/ML_Utils.ReturnMainStack` self) "/Game/UI/CAW_PauseMenu.CAW_PauseMenu_C"))
    (`WidgetBlueprintLibrary.SetInputMode_UIOnlyEx` self _returnvalue "DoNotLock" true)
    (set `self.bShowMouseCursor` true)
    (`self.SetMouseLocation` (`KismetMathLibrary.FTrunc` (/ _x 2.0)) (`KismetMathLibrary.FTrunc` (/ _y 2.0)))))

(event `EnhancedInput|/Game/Input/IA_DetectiveBoard`
  (params (ActionValue :type Boolean) (ElapsedSeconds :type "Float (double-precision)") (TriggeredSeconds :type "Float (double-precision)") (InputAction :type "InputAction Object Reference" :default "/Game/Input/IA_DetectiveBoard.IA_DetectiveBoard"))
  (bind _stack (`/Game/BP/Libraries/ML_Utils.ReturnMainStack` self))
  (:`Started`
    (bind _returnvalue (`CommonActivatableWidgetContainerBase.BP_AddWidget` _stack "/Game/UI/CAW_DetectiveBoard.CAW_DetectiveBoard_C"))
    (`WidgetBlueprintLibrary.SetInputMode_UIOnlyEx` self _returnvalue "DoNotLock" true)
    (set `self.bShowMouseCursor` true)
    (`self.OnDetectiveBoardOpen`)
    (`/Engine/EditorBlueprintResources/StandardMacros.DoOnce` false
      (:`Completed`
        (`CommonActivatableWidgetContainerBase.BP_AddWidget` _stack "/Game/UI/CAW_First_DetectiveTutorial.CAW_First_DetectiveTutorial_C")))))

(fn `UserConstructionScript`)